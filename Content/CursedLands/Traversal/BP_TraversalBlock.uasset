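; BP_TraversalBlock is a traversal obstacle that exposes four ledge splines and labels its height.
; The construction script stores the actor transform and sets a text label showing Z scale in meters, sized from the smaller of Y and Z scale.
; It also builds a ledge spline array and a map pairing each ledge with its opposite (front/back, right/left).
; Event graph logic is empty.
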(event EventBeginPlay)

(event Collision|EventActorBeginOverlap
  (params (OtherActor :type Actor%20Object%20Reference)))

(event EventTick
  (params (DeltaSeconds :type Float%20%28single-precision%29)))

(fn ConstructionScript
  (Variables|Default|SetInitialTransform (Transformation|GetActorTransform))
  (CallFunction|UpdateTexts)
  (Variables|Default|SetLedgeSplineComponents (Utilities|Array|MakeArray (Variables|Default|GetLedge_Front) (Variables|Default|GetLedge_Back) (Variables|Default|GetLedge_Right) (Variables|Default|GetLedge_Left)))
  (Variables|Default|SetOppositeLedgeSplineComponents (Utilities|Map|MakeMap (Variables|Default|GetLedge_Front) (Variables|Default|GetLedge_Back) (Variables|Default|GetLedge_Back) (Variables|Default|GetLedge_Front) (Variables|Default|GetLedge_Right) (Variables|Default|GetLedge_Left) (Variables|Default|GetLedge_Left) (Variables|Default|GetLedge_Right))))

(fn UpdateTexts
  (bind _initialtransform (Variables|Default|GetInitialTransform))
  (Rendering|Components|TextRender|SetText (Variables|Default|GetScaleFont) (Utilities|Text|FormatText "{Height}M" (Utilities|Text|ToText(Float) (.z (.scale (Variables|Default|GetInitialTransform))) "HalfToEven")))
  (Rendering|Components|TextRender|SetWorldSize (Variables|Default|GetScaleFont) (* (Math|Float|Min(Float) (.y (.scale _initialtransform)) (.z (.scale _initialtransform))) 2e+01)))