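; Player character gameplay ability that plays a heal montage and applies a healing gameplay effect to its owner.
; Once the montage starts, the ability waits for the heal cast gameplay tag, then commits, applies the effect and ends.
; Deferring the commit to the cast moment means cost and cooldown are not committed on activation.
; Montage blend out or interruption cancels the ability.
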(event Ability|EventActivateAbility
  (bind _returnvalue (Ability|GetAvatarActorfromActorInfo))
  (bind _aspawn (Utilities|Casting|CastToPawn _returnvalue))
  (Variables|Default|SetPlayerPawn _aspawn)
  (bind _ascl_player_character (Utilities|Casting|CastToCL_PlayerCharacter _returnvalue))
  (bind _output_get (Variables|Default|SetPlayerCharacter _ascl_player_character))
  (Variables|Default|SetPlayerCharacterAnimInstace (Components|SkeletalMesh|GetAnimInstance (Variables|/Script/Engine.Character|GetMesh _output_get)))
  (Animation|Montage|PlayMontage (Variables|/Script/Engine.Character|GetMesh _output_get) "/Game/CursedLands/Characters/PlayerCharacter/Animation/Attack/AM_PlayerCharacter_Heal.AM_PlayerCharacter_Heal" 1.0 0.0 "Default"
    (:then
      (Ability|Tasks|WaitGameplayTagAdd "(TagName=\"Gameplay.Ability.Heal.Cast\")" 0
        (:Added
          (Ability|CommitAbility)
          (Ability|ApplyGameplayEffectSpecToOwner (Ability|MakeOutgoingGameplayEffectSpec "/Game/CursedLands/Characters/PlayerCharacter/Gameplay/AbilitySystem/Effects/GE_PlayerCharacter_Heal.GE_PlayerCharacter_Heal_C"))
          (Ability|EndAbility))))
    (:OnBlendOut
      (Ability|CancelAbility :!label _label))
    (:OnInterrupted
      (goto _label))))

(event Ability|EventOnEndAbility
  (params (bWasCancelled :type Boolean)))