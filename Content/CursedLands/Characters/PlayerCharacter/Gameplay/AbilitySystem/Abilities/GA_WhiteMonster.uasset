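; GA_WhiteMonster is a player gameplay ability that plays a praying montage and applies the GE_WhiteMonster effect to its owner.
; Activation plays the montage on the character's anim instance and binds its section-changed and ended events.
; Reaching the "End" section applies the effect and only then commits the ability, so commit happens late and its result is unchecked.
; The montage-ended callback ends the ability, whether interrupted or not.
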(event Custom|OnPrayingMontageSectionChanged
  (params (Montage :type Anim%20Montage%20Object%20Reference) (SectionName :type Name) (bLooped :type Boolean))
  ;[0.1122 0 0.15 0.5] Praying Montage Callbacks
  (if (== SectionName "End")
    (GameplayEffects|ApplyGameplayEffectToSelf :self (Ability|GetAbilitySystemComponentfromActorInfo) :GameplayEffectClass "/Game/CursedLands/Characters/PlayerCharacter/Gameplay/AbilitySystem/Effects/GE_WhiteMonster.GE_WhiteMonster_C" :Level 1.0)
    (Ability|CommitAbility)))

(event Custom|OnPrayingMontageEnded
  (params (Montage :type Anim%20Montage%20Object%20Reference) (bInterrupted :type Boolean))
  ;[0.1122 0 0.15 0.5] Praying Montage Callbacks
  (Ability|EndAbility))

(event Ability|EventActivateAbility
  (bind _ascl_player_character (Utilities|Casting|CastToCL_PlayerCharacter (Ability|GetAvatarActorfromActorInfo)))
  (Animation|Montage|MontagePlay (Components|SkeletalMesh|GetAnimInstance (Variables|/Script/Engine.Character|GetMesh _ascl_player_character)) "/Game/CursedLands/Characters/PlayerCharacter/Animation/Abilities/AM_PlayerCharacter_Praying.AM_PlayerCharacter_Praying" 1.0 "MontageLength" 0.0 true)
  (EventDispatchers|BindEventtoOnMontageSectionChanged (Components|SkeletalMesh|GetAnimInstance (Variables|/Script/Engine.Character|GetMesh _ascl_player_character)) (EventDispatchers|CreateEvent :!event Custom|OnPrayingMontageSectionChanged))
  (EventDispatchers|BindEventtoOnMontageEnded (Components|SkeletalMesh|GetAnimInstance (Variables|/Script/Engine.Character|GetMesh _ascl_player_character)) (EventDispatchers|CreateEvent :!event Custom|OnPrayingMontageEnded)))

(event Ability|EventOnEndAbility
  (params (bWasCancelled :type Boolean)))