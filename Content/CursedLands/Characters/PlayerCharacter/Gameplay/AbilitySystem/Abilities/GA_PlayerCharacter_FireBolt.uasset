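; Player gameplay ability that casts a fire bolt projectile.
; After committing, it plays the aim-shoot montage from its Shoot section on the player mesh and waits for the Shooting gameplay tag to be added.
; The tag triggers spawning BP_FireBolt at the right cast socket, aimed by control rotation, then ends the ability.
; Failed commit or montage blend-out or interruption cancels it.
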(event Ability|EventActivateAbility
  (bind _returnvalue (Ability|GetAvatarActorfromActorInfo))
  (bind _returnvalue_2 (Ability|CommitAbility))
  (if _returnvalue_2
    (bind _aspawn (Utilities|Casting|CastToPawn _returnvalue))
    (Variables|Default|SetPlayerPawn _aspawn)
    (bind _ascl_player_character (Utilities|Casting|CastToCL_PlayerCharacter _returnvalue))
    (bind _output_get (Variables|Default|SetPlayerCharacter _ascl_player_character))
    (Variables|Default|SetPlayerCharacterAnimInstace (Components|SkeletalMesh|GetAnimInstance (Variables|/Script/Engine.Character|GetMesh _output_get)))
    (Animation|Montage|PlayMontage (Variables|/Script/Engine.Character|GetMesh _output_get) (Variables|Default|GetAimShootProjectileAnimMontage) 1.0 0.0 "Shoot"
      (:then
        (Ability|Tasks|WaitGameplayTagAdd "(TagName=\"Gameplay.Ability.ShootProjectile.Shooting\")" 0
          (:Added
            (Game|SpawnActorfromClass "/Game/CursedLands/Actors/Projectiles/FireBolt/BP_FireBolt.BP_FireBolt_C" (Math|Transform|MakeTransform (Transformation|GetSocketLocation (Variables|/Script/Engine.Character|GetMesh (Variables|Default|GetPlayerCharacter)) "Socket_CastRight") (Math|Rotator|MakeRotator 0.0 (.pitch (Pawn|GetControlRotation (Variables|Default|GetPlayerPawn) :!class /Script/Engine.Pawn)) (.yaw (Pawn|GetControlRotation (Variables|Default|GetPlayerPawn) :!class /Script/Engine.Pawn))) "1.000000,1.000000,1.000000") "AlwaysSpawn" "MultiplyWithRoot" (Ability|GetOwningActorfromActorInfo) (Variables|Default|GetPlayerPawn))
            (Ability|EndAbility))))
      (:OnBlendOut
        (Ability|CancelAbility :!label _label))
      (:OnInterrupted
        (goto _label)))
    (else
      (Ability|CancelAbility))))

(event Ability|EventOnEndAbility
  (params (bWasCancelled :type Boolean)))