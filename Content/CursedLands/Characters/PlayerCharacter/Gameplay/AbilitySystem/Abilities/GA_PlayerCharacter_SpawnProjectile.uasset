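; Gameplay ability that lets the player character shoot a BP_Projectile.
; If the cost check passes, it jumps the aim-shoot montage to its Shoot section and waits for the Shooting gameplay tag; otherwise it cancels.
; When the tag is added, it spawns the projectile at the owning actor's location using control-rotation yaw, then ends.
; CommitAbility is disconnected, so the ability checks cost but never commits it.
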(event Ability|EventActivateAbility
  (bind _returnvalue (Ability|GetOwningActorfromActorInfo))
  (bind _returnvalue_2 (Ability|GetAvatarActorfromActorInfo))
  (bind _returnvalue_3 (Class|GameplayAbility|CheckAbilityCost))
  (if _returnvalue_3
    (bind _aspawn (Utilities|Casting|CastToPawn _returnvalue_2))
    (Variables|Default|SetPlayerPawn _aspawn)
    (bind _ascl_player_character (Utilities|Casting|CastToCL_PlayerCharacter _returnvalue_2))
    (bind _output_get (Variables|Default|SetPlayerCharacter _ascl_player_character))
    (bind _output_get_2 (Variables|Default|SetPlayerCharacterAnimInstace (Components|SkeletalMesh|GetAnimInstance (Variables|/Script/Engine.Character|GetMesh _output_get))))
    (Ability|Animation|MontageJumptoSection _output_get_2 "Shoot" (Variables|Default|GetAimShootProjectileAnimMontage))
    (Ability|Tasks|WaitGameplayTagAdd "(TagName=\"Gameplay.Ability.ShootProjectile.Shooting\")" 0
      (:Added
        (Game|SpawnActorfromClass "/Game/Developers/Anton/Actors/Projectiles/BP_Projectile.BP_Projectile_C" (Math|Transform|MakeTransform (.location (Transformation|GetActorTransform _returnvalue)) (Math|Rotator|MakeRotator 0.0 0.0 (.yaw (Pawn|GetControlRotation (Variables|Default|GetPlayerPawn) :!class /Script/Engine.Pawn))) "1.000000,1.000000,1.000000") "AlwaysSpawn" "MultiplyWithRoot" _returnvalue (Variables|Default|GetPlayerPawn))
        (Ability|EndAbility)))
    (else
      (Ability|CancelAbility))))

(event Ability|EventOnEndAbility
  (params (bWasCancelled :type Boolean)))