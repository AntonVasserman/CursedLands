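; Gameplay ability that makes the player character dodge forward, back, left or right.
; After committing, it adds a local dodging tag and uses Motion Matching against pose history to pick one of four directional montages.
; The chosen montage's direction sets a Motion Warping target a fixed distance along the actor's forward or right axis, then it plays slightly sped up.
; The ability ends when the montage finishes, blends out or is interrupted, removing the tag.
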(event Ability|EventActivateAbility
  (bind _returnvalue (Ability|CommitAbility))
  (if _returnvalue
    (bind _ascl_player_character (Utilities|Casting|CastToCL_PlayerCharacter (Game|GetPlayerCharacter 0))
      (:then
        (Variables|Default|SetPlayerCharacter _ascl_player_character)
        (Ability|GameplayEffect|AddLooseGameplayTags (Variables|Default|GetPlayerCharacter) (GameplayTags|MakeLiteralGameplayTagContainer "(GameplayTags=((TagName=\"Locomotion.Dodging\")))"))
        (bind _asanim_montage (Utilities|Casting|CastToAnimMontage (.selectedanim (Class|PoseSearchLibrary|MotionMatch (Components|SkeletalMesh|GetAnimInstance (Variables|/Script/Engine.Character|GetMesh (Variables|Default|GetPlayerCharacter))) (Utilities|Array|MakeArray "/Game/CursedLands/Characters/PlayerCharacter/Animation/Dodge/AM_PlayerCharacter_Dodge_B.AM_PlayerCharacter_Dodge_B" "/Game/CursedLands/Characters/PlayerCharacter/Animation/Dodge/AM_PlayerCharacter_Dodge_F.AM_PlayerCharacter_Dodge_F" "/Game/CursedLands/Characters/PlayerCharacter/Animation/Dodge/AM_PlayerCharacter_Dodge_L.AM_PlayerCharacter_Dodge_L" "/Game/CursedLands/Characters/PlayerCharacter/Animation/Dodge/AM_PlayerCharacter_Dodge_R.AM_PlayerCharacter_Dodge_R") "PoseHistory")))
          (:then
            (Variables|Default|SetChosenAnimMontage _asanim_montage)
            (Class|MotionWarpingComponent|AddorUpdateWarpTargetfromLocation (Class|CLPlayerCharacter|GetMotionWarping (Variables|Default|GetPlayerCharacter)) "Target" (+ (Transformation|GetActorLocation (Variables|Default|GetPlayerCharacter)) (* (Math|Vector|SelectVector (Transformation|GetActorForwardVector (Variables|Default|GetPlayerCharacter)) (Transformation|GetActorRightVector (Variables|Default|GetPlayerCharacter)) (or (== (Variables|Default|GetChosenAnimMontage) "/Game/CursedLands/Characters/PlayerCharacter/Animation/Dodge/AM_PlayerCharacter_Dodge_B.AM_PlayerCharacter_Dodge_B") (== (Variables|Default|GetChosenAnimMontage) "/Game/CursedLands/Characters/PlayerCharacter/Animation/Dodge/AM_PlayerCharacter_Dodge_F.AM_PlayerCharacter_Dodge_F"))) (* (Math|Float|MakeLiteralFloat 2.5e+02) (Math|Float|SelectFloat 1.0 -1.0 (or (== (Variables|Default|GetChosenAnimMontage) "/Game/CursedLands/Characters/PlayerCharacter/Animation/Dodge/AM_PlayerCharacter_Dodge_F.AM_PlayerCharacter_Dodge_F") (== (Variables|Default|GetChosenAnimMontage) "/Game/CursedLands/Characters/PlayerCharacter/Animation/Dodge/AM_PlayerCharacter_Dodge_R.AM_PlayerCharacter_Dodge_R")))))))
            (Animation|Montage|PlayMontage (Variables|/Script/Engine.Character|GetMesh (Variables|Default|GetPlayerCharacter)) (Variables|Default|GetChosenAnimMontage) 1.25
              (:OnCompleted
                _)
              (:OnBlendOut
                _)
              (:OnInterrupted
                _))
            (Ability|EndAbility))
          (:CastFailed
            (Ability|EndAbility))))
      (:CastFailed
        (Ability|EndAbility :!label _label)))
    (else
      (goto _label))))

(event Ability|EventOnEndAbility
  (params (bWasCancelled :type Boolean))
  (Ability|GameplayEffect|RemoveLooseGameplayTags (Variables|Default|GetPlayerCharacter) (GameplayTags|MakeLiteralGameplayTagContainer "(GameplayTags=((TagName=\"Locomotion.Dodging\")))")))