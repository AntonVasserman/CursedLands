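; Gameplay ability that puts the player character into an aiming state while its input is held.
; On activation it casts the avatar to CL_PlayerCharacter and plays the aim-shoot montage on the mesh's anim instance.
; A WaitInputRelease task ends the ability when the input is released, and ending stops the montage using the montage's own blend-out time.
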(event Ability|EventActivateAbility
  (bind _ascl_player_character (Utilities|Casting|CastToCL_PlayerCharacter (Ability|GetAvatarActorfromActorInfo)))
  (Variables|Default|SetPlayerCharacterAnimInstace (Components|SkeletalMesh|GetAnimInstance (Variables|/Script/Engine.Character|GetMesh _ascl_player_character)))
  (Animation|Montage|MontagePlay (Variables|Default|GetPlayerCharacterAnimInstace) (Variables|Default|GetAimShootMontage) 1.0 "MontageLength" 0.0 true)
  (Ability|Tasks|WaitInputRelease false
    (:OnRelease
      (Ability|EndAbility))))

(event Ability|EventOnEndAbility
  (params (bWasCancelled :type Boolean))
  (bind _aimshootmontage (Variables|Default|GetAimShootMontage))
  (Animation|Montage|MontageStop (Variables|Default|GetPlayerCharacterAnimInstace) (.blendtime (Class|AnimMontage|GetBlendOutArgs _aimshootmontage)) _aimshootmontage))