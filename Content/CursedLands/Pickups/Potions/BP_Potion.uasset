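; BP_Potion is a Health or Mana pickup that applies a gameplay effect to the player who overlaps it.
; The construction script uses the Type enum to choose the mesh material, gameplay effect and idle Niagara color.
; Each tick bobs the potion on a sine wave around its spawn location and spins it around a configurable axis.
; On overlap it applies the effect through GAS, spawns a color-matched collect effect, plays a sound and destroys itself.
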(event OnComponentBeginOverlap(Sphere)
  (params (OverlappedComponent :type Primitive%20Component%20Object%20Reference) (OtherActor :type Actor%20Object%20Reference) (OtherComp :type Primitive%20Component%20Object%20Reference) (OtherBodyIndex :type Integer) (bFromSweep :type Boolean) (SweepResult :type Hit%20Result%20Structure%20%28by%20ref%29))
  (bind _ascl_player_character (Utilities|Casting|CastToCL_PlayerCharacter OtherActor))
  (GameplayEffects|ApplyGameplayEffectToSelf :self (Ability|GetAbilitySystemComponent _ascl_player_character) :GameplayEffectClass (Variables|Default|GetGameplayEffect) :Level 1.0)
  (bind _returnvalue (Niagara|SpawnSystematLocation "/Game/CursedLands/Pickups/Potions/FX/NS_Potion_Collect.NS_Potion_Collect" (Transformation|GetActorLocation)))
  (Niagara|SetNiagaraVariable(LinearColor) _returnvalue "Color" (* (Utilities|Select :Index (Variables|Default|GetType) :NewEnumerator0 (Variables|Defaults|GetHealthIdleEffectColor) :NewEnumerator1 (Variables|Defaults|GetManaIdleEffectColor)) (Math|Float|MakeLiteralFloat 1e+02)))
  (Audio|PlaySoundatLocation "/Game/CursedLands/Pickups/Potions/Audio/MSS_Potion.MSS_Potion" (Transformation|GetActorLocation) "0, 0, 0" 1.0 1.0 0.0 0 0 0 0)
  (Actor|DestroyActor))

(event EventBeginPlay
  (Variables|Default|SetInitialTransform (Transformation|GetActorTransform)))

(event EventTick
  (params (DeltaSeconds :type Float%20%28single-precision%29))
  (CallFunction|TickFloating DeltaSeconds)
  (CallFunction|TickRotation DeltaSeconds))

(fn ConstructionScript
  (Rendering|Material|SetMaterial (Variables|Debug|GetStaticMeshComponent) 0 (Utilities|Select :Index (Variables|Default|GetType) :NewEnumerator0 (Variables|Defaults|GetHealthMaterialInstance) :NewEnumerator1 (Variables|Defaults|GetManaMaterialInstance)))
  (Variables|Default|SetGameplayEffect (Utilities|Select :Index (Variables|Default|GetType) :NewEnumerator0 (Variables|Defaults|GetHealthGameplayEffect) :NewEnumerator1 (Variables|Defaults|GetManaGameplayEffect)))
  (Niagara|SetNiagaraVariable(LinearColor) (Variables|Default|GetIdleEffect) "Color" (* (Utilities|Select :Index (Variables|Default|GetType) :NewEnumerator0 (Variables|Defaults|GetHealthIdleEffectColor) :NewEnumerator1 (Variables|Defaults|GetManaIdleEffectColor)) (Math|Float|MakeLiteralFloat 1e+02))))

(fn TickFloating
  (params (DeltaSeconds :type Float%20%28double-precision%29))
  (bind _initialtransform (Variables|Default|GetInitialTransform))
  (Variables|Floating|SetFloatingElapsedTime (+ (Variables|Floating|GetFloatingElapsedTime) (* DeltaSeconds (Variables|Floating|GetFloatingSpeed))))
  (if (> (Variables|Floating|GetFloatingElapsedTime) (* (Math|Trig|GetPI) 2.0))
    (Variables|Floating|SetFloatingElapsedTime (- (Variables|Floating|GetFloatingElapsedTime) (* (Math|Trig|GetPI) 2.0))))
  (Transformation|SetActorLocation (Math|Vector|MakeVector (.x (.location _initialtransform)) (.y (.location _initialtransform)) (+ (.z (.location _initialtransform)) (* (Math|Trig|Sin(Radians) (Variables|Floating|GetFloatingElapsedTime)) (Variables|Floating|GetFloatingAmplitude)))) false false))

(fn TickRotation
  (params (DeltaSeconds :type Float%20%28double-precision%29))
  (bind _rotationspeed (Variables|Rotation|GetRotationSpeed))
  (bind _rotationaxis (Variables|Rotation|GetRotationAxis))
  (bind _returnvalue (* _rotationspeed 1e+02))
  (bind _returnvalue_2 (* DeltaSeconds _returnvalue))
  (bind _returnvalue_3 (* _rotationaxis _returnvalue_2))
  (Transformation|AddActorLocalRotation (Math|Rotator|MakeRotator (.x _returnvalue_3) (.y _returnvalue_3) (.z _returnvalue_3)) false false))