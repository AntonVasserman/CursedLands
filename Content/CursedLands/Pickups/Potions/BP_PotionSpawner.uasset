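; Potion spawner pickup point that spawns a health or mana potion and respawns it after the potion is destroyed.
; BeginPlay spawns at once without effects or starts an initial delay, and Tick counts down a timer that triggers delayed spawns with sound and a type-tinted Niagara effect.
; The potion's destroyed event restarts that timer with the respawn delay.
; The construction script colors the base material by potion type.
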(event EventBeginPlay
  (if (== (Variables|Config|GetInitialSpawnDelay) 0.0)
    (CallFunction|SpawnPotion false)
    (else
      (Variables|Default|SetRespawnTimer (Math|Float|Max(Float) (Variables|Config|GetInitialSpawnDelay) 0.0)))))

(event EventTick
  (params (DeltaSeconds :type Float%20%28single-precision%29))
  (if (>= (Variables|Default|GetRespawnTimer) 0.0)
    (bind _output_get (Variables|Default|SetRespawnTimer (- (Variables|Default|GetRespawnTimer) DeltaSeconds)))
    (if (< _output_get 0.0)
      (CallFunction|SpawnPotion true))))

(fn ConstructionScript
  (Rendering|Material|SetMaterial (Variables|Default|GetInnerBase) 0 (Utilities|Select :Index (Variables|Config|GetPotionType) :NewEnumerator0 "/AVLevelPrototyping/AVLevelPrototyping/Materials/Grid/MI_Grid_Red.MI_Grid_Red" :NewEnumerator1 "/AVLevelPrototyping/AVLevelPrototyping/Materials/Grid/MI_Grid_Blue.MI_Grid_Blue")))

(fn SpawnPotion
  (params (bPlaySpawnSound :type Boolean))
  (bind _returnvalue (Game|SpawnActorfromClass "/Game/CursedLands/Pickups/Potions/BP_Potion.BP_Potion_C" (Math|Transform|MakeTransform (Transformation|GetWorldLocation (Variables|Default|GetPotionSpawnLocation)) "0, 0, 0" "1.000000,1.000000,1.000000") "AlwaysSpawn" "MultiplyWithRoot" 0 (Variables|Config|GetPotionType) 0))
  (Game|BindEventtoOnDestroyed _returnvalue (EventDispatchers|CreateEvent :!event SpawnedPotiononDestrotyed))
  (if bPlaySpawnSound
    (Audio|PlaySoundatLocation "/Game/CursedLands/Pickups/Potions/Audio/MSS_Potion_Spawn_P.MSS_Potion_Spawn_P" (+ (Transformation|GetWorldLocation (Variables|Default|GetPotionSpawnLocation)) "0.000000,0.000000,50.000000") "0, 0, 0" 1.0 1.0 0.0 0 0 0 0)
    (bind _returnvalue_2 (Niagara|SpawnSystematLocation "/Game/CursedLands/Pickups/Potions/FX/NS_Potion_Spawn.NS_Potion_Spawn" (Transformation|GetWorldLocation (Variables|Default|GetPotionSpawnLocation))))
    (Niagara|SetNiagaraVariable(LinearColor) _returnvalue_2 "Color" (* (Utilities|Select :Index (Variables|Config|GetPotionType) :NewEnumerator0 (Variables|Defaults|GetHealthSpawnEffectColor) :NewEnumerator1 (Variables|Defaults|GetManaSpawnEffectColor)) (Math|Float|MakeLiteralFloat 1e+02)))))

(fn SpawnedPotiononDestrotyed
  (params (DestroyedActor :type Actor%20Object%20Reference))
  (Variables|Default|SetRespawnTimer (Variables|Config|GetRespawnDelay)))