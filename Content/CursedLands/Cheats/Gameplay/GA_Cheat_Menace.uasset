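; Gameplay ability for the Menace cheat, which plays a menacing montage on the player character.
; While the montage plays, each addition of the Cast gameplay tag commits the ability, applies the Menace gameplay effect to the owner and spawns a Niagara effect just above the character's location.
; Montage completion ends the ability, while blend out or interruption cancels it, and all three deactivate the Niagara effect.
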(event Ability|EventActivateAbility
  (bind _returnvalue (Ability|GetAvatarActorfromActorInfo))
  (bind _aspawn (Utilities|Casting|CastToPawn _returnvalue))
  (Variables|Default|SetPlayerPawn _aspawn)
  (bind _ascl_player_character (Utilities|Casting|CastToCL_PlayerCharacter _returnvalue))
  (bind _output_get (Variables|Default|SetPlayerCharacter _ascl_player_character))
  (Variables|Default|SetPlayerCharacterAnimInstace (Components|SkeletalMesh|GetAnimInstance (Variables|/Script/Engine.Character|GetMesh _output_get)))
  (Animation|Montage|PlayMontage (Variables|/Script/Engine.Character|GetMesh _output_get) "/Game/CursedLands/Cheats/Animation/Montages/AM_PlayerCharacter_Menacing.AM_PlayerCharacter_Menacing" 1.0 0.0 "Default"
    (:then
      (Ability|Tasks|WaitGameplayTagAdd "(TagName=\"Gameplay.Ability.Menace.Cast\")" 0
        (:Added
          (Ability|CommitAbility)
          (Ability|ApplyGameplayEffectSpecToOwner (Ability|MakeOutgoingGameplayEffectSpec "/Game/CursedLands/Cheats/Gameplay/GE_Cheat_Menace.GE_Cheat_Menace_C"))
          (bind _returnvalue_2 (Niagara|SpawnSystematLocation "/Game/CursedLands/Cheats/VFX/NS_Cheat_Menace.NS_Cheat_Menace" (+ (Transformation|GetActorLocation (Variables|Default|GetPlayerCharacter)) "0.000000,0.000000,50.000000")))
          (Variables|Default|SetEffect _returnvalue_2))))
    (:OnCompleted
      (Ability|EndAbility)
      (bind _effect (Variables|Default|GetEffect :!label _label)
        (:then
          (Components|Activation|Deactivate _effect))
        (:else)))
    (:OnBlendOut
      (Ability|CancelAbility :!label _label_2)
      (goto _label))
    (:OnInterrupted
      (goto _label_2))))