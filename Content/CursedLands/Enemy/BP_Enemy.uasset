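; Enemy Blueprint for Cursed Lands with a world-space health bar that appears when health changes.
; On BeginPlay it caches the player and bar widget, hides the bar, binds HealthComponent events, and passes the health view model to the widget once instantiated.
; Health changes show the bar and restart its fade-out animation.
; Tick turns the bar toward the player's gameplay camera, and DieBP destroys the actor.
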(event Custom|OnHealthViewModelInstantiated
  (params (ResourceViewModel :type CL%20Resource%20View%20Model%20Object%20Reference))
  (Default|SetHealthViewModel (Variables|Default|GetHealthBarWidget) ResourceViewModel))

(event EventDieBP
  (Actor|DestroyActor))

(event EventBeginPlay
  (bind _ascl_player_character (Utilities|Casting|CastToCL_PlayerCharacter (Game|GetPlayerCharacter 0)))
  (Variables|Default|SetCLPlayerCharacter _ascl_player_character)
  (bind _aswbp_enemy_health_bar (Utilities|Casting|CastToWBP_EnemyHealthBar (UserInterface|GetWidget (Variables|Default|GetHealthWidget))))
  (Variables|Default|SetHealthBarWidget _aswbp_enemy_health_bar)
  (EventDispatchers|BindEventtoOnResourceViewModelInstantiated (Variables|Default|GetHealthComponent) (delegate Custom|OnHealthViewModelInstantiated))
  (EventDispatchers|BindEventtoOnResourceValueChanged (Variables|Default|GetHealthComponent) (EventDispatchers|CreateEvent :!event OnHealthValueChanged))
  (Rendering|SetVisibility (Variables|Default|GetHealthWidget) false false))

(event EventTick
  (params (DeltaSeconds :type Float%20%28single-precision%29))
  (Transformation|SetWorldRotation (Variables|Default|GetHealthWidget) (Math|Rotator|FindLookatRotation (Transformation|GetWorldLocation (Variables|Default|GetHealthWidget)) (Transformation|GetWorldLocation (Variables|/Script/CursedLands.CL_PlayerCharacter|GetGameplayCamera (Variables|Default|GetCLPlayerCharacter)))) false false))

(fn ConstructionScript)

(fn OnHealthValueChanged
  (params (NewHealth :type Integer))
  (Rendering|SetVisibility (Variables|Default|GetHealthWidget) true false)
  (Class|UserWidget|StopAnimation (Variables|Default|GetHealthBarWidget) (Variables|/Game/Developers/Anton/UI/Enemies/WBP_EnemyHealthBar.WBP_EnemyHealthBar_C|GetFadeOut (Variables|Default|GetHealthBarWidget)))
  (UserInterface|Animation|PlayAnimation (Variables|Default|GetHealthBarWidget) (Variables|/Game/Developers/Anton/UI/Enemies/WBP_EnemyHealthBar.WBP_EnemyHealthBar_C|GetFadeOut (Variables|Default|GetHealthBarWidget)) 0.0 1 "Forward" 1.0 false))