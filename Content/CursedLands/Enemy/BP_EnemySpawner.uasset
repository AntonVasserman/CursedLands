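; BP_EnemySpawner is an actor that spawns a limited number of BP_Enemy actors at its SpawnLocation, starting at BeginPlay after an optional initial delay.
; Further spawns follow on a respawn timer, or only after a spawned enemy is destroyed when RespawnOnDeathOnly is set.
; It fires dispatchers when a spawned enemy is destroyed and when the count is depleted.
; ResetSpawner sets a new total, clears the count and can reactivate it.
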(event Custom|SpawnEnemy
  ;[0.1221 0.3095 0.09084 0.502] Guard
  (if (!= (Variables|Default|GetCurrentSpawnCount) (Variables|Config|GetTotalSpawnCount))
    (bind _returnvalue (Game|SpawnActorfromClass "/Game/CursedLands/Enemy/BP_Enemy.BP_Enemy_C" (Math|Transform|MakeTransform (Transformation|GetWorldLocation (Variables|Default|GetSpawnLocation)) "0, 0, 0" "1.000000,1.000000,1.000000") "AdjustIfPossibleButAlwaysSpawn" "MultiplyWithRoot" 0 0))
    (Game|AssignOnDestroyed _returnvalue (EventDispatchers|CreateEvent :!event Custom|SpawnedEnemy_OnDestroyed))
    (Math|Integer|IncrementInt (Variables|Default|GetCurrentSpawnCount)
      (:%20%20
        ;[0.1221 0.3095 0.09084 0.502] Guard
        (if (!= (Variables|Default|GetCurrentSpawnCount) (Variables|Config|GetTotalSpawnCount))
          (if (not (Variables|Config|GetbRespawnOnDeathOnly))
            (Utilities|Time|SetTimerbyEvent (EventDispatchers|CreateEvent :!event Custom|SpawnEnemy) (Variables|Config|GetRespawnDelay)))
          (else
            (Default|CallOnSpawnerDepleted self)))))))

(event Custom|SpawnedEnemy_OnDestroyed
  (params (DestroyedActor :type Actor%20Object%20Reference))
  (Utilities|FlowControl|Sequence
    (:then_0
      (if (Variables|Config|GetbRespawnOnDeathOnly)
        (Utilities|Time|SetTimerbyEvent (EventDispatchers|CreateEvent :!event Custom|SpawnEnemy) (Variables|Config|GetRespawnDelay))))
    (:then_1
      (Default|CallOnSpawnedEnemyDestroyed))))

(event EventBeginPlay
  (CallFunction|ActivateSpawner))

(fn ConstructionScript)

(fn ResetSpawner
  (params (TotalSpawnCount :type Integer) (bActivate :type Boolean))
  (Variables|Config|SetTotalSpawnCount TotalSpawnCount)
  (Variables|Default|SetCurrentSpawnCount 0)
  (if bActivate
    (CallFunction|ActivateSpawner)))

(fn ActivateSpawner
  (if (<= (Variables|Config|GetInitialSpawnDelay) 0.0)
    (CallFunction|SpawnEnemy)
    (else
      (Utilities|Time|SetTimerbyEvent (EventDispatchers|CreateEvent :!event Custom|SpawnEnemy) (Variables|Config|GetInitialSpawnDelay)))))