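; BP_Enemy_Exploder is the Exploder enemy in Cursed Lands, whose look and speed depend on the game difficulty.
; On BeginPlay it reads the difficulty from the local user settings (CL_GameLocalUserSettings).
; It then swaps both mesh materials, body and lava drip, and sets a faster walk speed on Hard.
; No explosion or AI logic lives in this graph, and its Tick and overlap events are disabled.
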(event EventBeginPlay
  (|CallParentFunction)
  (Utilities|FlowControl|Sequence
    (:then_0
      (bind _returnvalue (Settings|GetGameUserSettings))
      (bind _ascl_game_local_user_settings (Utilities|Casting|CastToCL_GameLocalUserSettings _returnvalue))
      (Variables|Default|SetLocalUserSettings _ascl_game_local_user_settings)
      (Variables|Default|SetGameDifficulty (Class|CLGameLocalUserSettings|GetDifficulty (Variables|Default|GetLocalUserSettings))))
    (:then_1
      (Rendering|Material|SetMaterial (Variables|Character|GetMesh) 0 (Utilities|Select :Index (Variables|Default|GetGameDifficulty) :Normal "/Game/CursedLands/Enemies/Exploder/Materials/M_Exploder.M_Exploder" :Hard "/Game/CursedLands/Enemies/Exploder/Materials/M_Exploder_Hard.M_Exploder_Hard"))
      (Rendering|Material|SetMaterial (Variables|Character|GetMesh) 1 (Utilities|Select :Index (Variables|Default|GetGameDifficulty) :Normal "/Game/CursedLands/Enemies/Exploder/Materials/M_Exploder_LavaDrip.M_Exploder_LavaDrip" :Hard "/Game/CursedLands/Enemies/Exploder/Materials/M_Exploder_LavaDrip_Hard.M_Exploder_LavaDrip_Hard"))
      (Variables|/Script/Engine.CharacterMovementComponent|SetMaxWalkSpeed (Variables|Character|GetCharacterMovement) (Utilities|Select :Index (Variables|Default|GetGameDifficulty) :Normal 4e+02 :Hard 6e+02)))))

(event Collision|EventActorBeginOverlap
  (params (OtherActor :type Actor%20Object%20Reference)))

(event EventTick
  (params (DeltaSeconds :type Float%20%28single-precision%29))
  (|CallParentFunction DeltaSeconds) ; This node is disabled and will not be called.\nDrag off pins to build functionality.
)

(fn ConstructionScript
  (|CallParentFunction))