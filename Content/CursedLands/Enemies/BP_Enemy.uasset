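; Enemy character that deals area damage with an attack or a self-destructing explosion, which also adds score.
; Attack applies a damage effect to characters in the impact capsule, knocks back a non-invulnerable player with brief invulnerability, and hides the indicator decal.
; A camera-facing health bar binds to the health component's view model and fades after changes.
; It optionally plays a spawn montage and mirrors the player's Menace cheat tag as its Stunned tag.
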(event Custom|StartIndicator
  (Rendering|SetVisibility (Variables|Default|GetDecal) true false))

(event Custom|Explode
  (Utilities|FlowControl|Sequence
    (:then_0
      (for _array_element (Collision|GetOverlappingActors (Variables|Default|GetExplosionImpactCapsule) "/Script/CursedLands.CL_Character" :!class /Script/Engine.PrimitiveComponent)
        (if (!= _array_element self)
          (Utilities|IsValid (Actor|GetComponentbyClass _array_element "/Script/CursedLands.CL_HealthComponent")
            (:Is%20Valid
              (GameplayEffects|ApplyGameplayEffectToTarget :self (Ability|GetAbilitySystemComponent 0) :GameplayEffectClass "/Game/CursedLands/Enemies/Gameplay/AbilitySystem/Effects/GE_Enemy_ExplodeDamage.GE_Enemy_ExplodeDamage_C" :Target (Ability|GetAbilitySystemComponent _array_element) :Level 1.0)
              (if (== _array_element (Game|GetPlayerCharacter 0))
                (if (not (GameplayTags|HasMatchingGameplayTag (Ability|GetAbilitySystemComponent (Game|GetPlayerCharacter 0)) "(TagName=\"Gameplay.Buff.Invulnerability\")"))
                  (Physics|AddImpulse (Variables|/Script/Engine.Character|GetCharacterMovement (Game|GetPlayerCharacter 0)) (* (- (Transformation|GetActorLocation (Game|GetPlayerCharacter 0)) (Transformation|GetActorLocation)) (Math|Conversions|ToVector(Float) 5e+02)) false)
                  (GameplayEffects|ApplyGameplayEffectToTarget :self (Ability|GetAbilitySystemComponent 0) :GameplayEffectClass "/Game/CursedLands/Enemies/Gameplay/AbilitySystem/Effects/GE_Invulnerability.GE_Invulnerability_C" :Target (Ability|GetAbilitySystemComponent (Game|GetPlayerCharacter 0)) :Level 1.0)))))))
      (Rendering|SetVisibility (Variables|Default|GetDecal) false false))
    (:then_1
      (Class|CLScoreSubsystem|AddScore (Subsystems|GetCLScoreSubsystem) 100)
      (Actor|DestroyActor))))

(event Custom|Attack
  (for _array_element (Collision|GetOverlappingActors (Variables|Default|GetExplosionImpactCapsule) "/Script/CursedLands.CL_Character" :!class /Script/Engine.PrimitiveComponent)
    (if (!= _array_element self)
      (Utilities|IsValid (Actor|GetComponentbyClass _array_element "/Script/CursedLands.CL_HealthComponent")
        (:Is%20Valid
          (GameplayEffects|ApplyGameplayEffectToTarget :self (Ability|GetAbilitySystemComponent 0) :GameplayEffectClass "/Game/CursedLands/Enemies/Gameplay/AbilitySystem/Effects/GE_Enemy_ExplodeDamage.GE_Enemy_ExplodeDamage_C" :Target (Ability|GetAbilitySystemComponent _array_element) :Level 1.0)
          (if (== _array_element (Game|GetPlayerCharacter 0))
            (if (not (GameplayTags|HasMatchingGameplayTag (Ability|GetAbilitySystemComponent (Game|GetPlayerCharacter 0)) "(TagName=\"Gameplay.Buff.Invulnerability\")"))
              (Physics|AddImpulse (Variables|/Script/Engine.Character|GetCharacterMovement (Game|GetPlayerCharacter 0)) (* (- (Transformation|GetActorLocation (Game|GetPlayerCharacter 0)) (Transformation|GetActorLocation)) (Math|Conversions|ToVector(Float) 5e+02)) false)
              (GameplayEffects|ApplyGameplayEffectToTarget :self (Ability|GetAbilitySystemComponent 0) :GameplayEffectClass "/Game/CursedLands/Enemies/Gameplay/AbilitySystem/Effects/GE_Invulnerability.GE_Invulnerability_C" :Target (Ability|GetAbilitySystemComponent (Game|GetPlayerCharacter 0)) :Level 1.0)))))))
  (Rendering|SetVisibility (Variables|Default|GetDecal) false false))

(event Custom|OnHealthViewModelInstantiated
  (params (ResourceViewModel :type CL%20Resource%20View%20Model%20Object%20Reference))
  (Default|SetHealthViewModel (Variables|Default|GetHealthBarWidget) ResourceViewModel))

(event EventBeginPlay
  (Utilities|FlowControl|Sequence
    (:then_0
      (bind _ascl_player_character (Utilities|Casting|CastToCL_PlayerCharacter (Game|GetPlayerCharacter 0)))
      (Variables|Default|SetCLPlayerCharacter _ascl_player_character)
      (bind _aswbp_enemy_health_bar (Utilities|Casting|CastToWBP_EnemyHealthBar (UserInterface|GetWidget (Variables|Default|GetHealthWidget))))
      (Variables|Default|SetHealthBarWidget _aswbp_enemy_health_bar)
      (EventDispatchers|BindEventtoOnResourceViewModelInstantiated (Class|CLCharacter|GetHealthComponent) (delegate Custom|OnHealthViewModelInstantiated))
      (EventDispatchers|BindEventtoOnResourceValueChanged (Class|CLCharacter|GetHealthComponent) (EventDispatchers|CreateEvent :!event OnHealthValueChanged))
      (Rendering|SetVisibility (Variables|Default|GetHealthWidget) false false)
      (Ability|Tasks|WaitGameplayTagAddToActor (Game|GetPlayerCharacter 0) "(TagName=\"Cheat.Ability.Menace\")"
        (:then
          (Ability|Tasks|WaitGameplayTagRemoveFromActor (Game|GetPlayerCharacter 0) "(TagName=\"Cheat.Ability.Menace\")"
            (:Removed
              (Ability|GameplayEffect|RemoveLooseGameplayTags self (GameplayTags|MakeGameplayTagContainerfromTag "(TagName=\"Enemy.State.Stunned\")")))))
        (:Added
          (Ability|GameplayEffect|AddLooseGameplayTags self (GameplayTags|MakeGameplayTagContainerfromTag "(TagName=\"Enemy.State.Stunned\")")))))
    (:then_1
      (if (Variables|Config|GetbPlaySpawnAnimation)
        (Animation|PlayAnimMontage (Variables|Config|GetSpawnAnimMontage) 1.0 "None")))))

(event EventTick
  (params (DeltaSeconds :type Float%20%28single-precision%29))
  (Transformation|SetWorldRotation (Variables|Default|GetHealthWidget) (Math|Rotator|FindLookatRotation (Transformation|GetWorldLocation (Variables|Default|GetHealthWidget)) (Transformation|GetWorldLocation (Variables|/Script/CursedLands.CL_PlayerCharacter|GetGameplayCamera (Variables|Default|GetCLPlayerCharacter)))) false false))

(fn ConstructionScript)

(fn OnHealthValueChanged
  (params (NewHealth :type Integer))
  (Rendering|SetVisibility (Variables|Default|GetHealthWidget) true false)
  (Class|UserWidget|StopAnimation (Variables|Default|GetHealthBarWidget) (Variables|/Game/Developers/Anton/UI/Enemies/WBP_EnemyHealthBar.WBP_EnemyHealthBar_C|GetFadeOut (Variables|Default|GetHealthBarWidget)))
  (UserInterface|Animation|PlayAnimation (Variables|Default|GetHealthBarWidget) (Variables|/Game/Developers/Anton/UI/Enemies/WBP_EnemyHealthBar.WBP_EnemyHealthBar_C|GetFadeOut (Variables|Default|GetHealthBarWidget)) 0.0 1 "Forward" 1.0 false))