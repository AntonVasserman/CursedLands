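; BP_Example is an example Blueprint that sets the DoOnce macro beside a hand-built equivalent, with no clear gameplay role.
; WithMacro gates a call to the empty SomeLogic function through DoOnce.
; WithoutMacro rebuilds that gate from a Sequence, branches and the Initialized and Closed flags, including the StartClosed option.
; Its reset logic, which reopens the gate, is present but unconnected.
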(fn WithMacro
  (Utilities|FlowControl|DoOnce false
    (:Completed
      (CallFunction|SomeLogic))))

(fn WithoutMacro
  ;[0.15 0.15 0.15 0.5] Do Once
  (LocalVariables|SetbStartClosed false)
  (Utilities|FlowControl|Sequence
    (:then_0
      (if (not (LocalVariables|GetbInitialized))
        (LocalVariables|SetbInitialized true)
        (if (LocalVariables|GetbStartClosed)
          (LocalVariables|SetbClosed true))))
    (:then_1
      (if (not (LocalVariables|GetbClosed))
        (LocalVariables|SetbClosed true)
        (CallFunction|SomeLogic)))))

(fn SomeLogic)